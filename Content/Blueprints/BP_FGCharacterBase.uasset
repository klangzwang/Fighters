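; Base character Blueprint for a side-on fighting game, handling movement on a fixed 2D plane and pushing between fighters.
; Tick snaps Y to zero, and capsule hits while walking nudge an idle opponent along X by facing direction.
; Events toggle WorldDynamic collision, flash named floor spotlights via timeline, and apply launches.
; Jump, mesh-shake and per-level character lighting logic is disconnected, and HitShaking is empty.
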(event `self.CapsuleComponent.OnComponentHit`
  (params (HitComponent :type "PrimitiveComponent Object Reference") (OtherActor :type "Actor Object Reference") (OtherComp :type "PrimitiveComponent Object Reference") (NormalImpulse :type "Vector Structure") (Hit :type "HitResult Structure (by ref)"))
  (bind _movestate (`self.moveState`))
  (if (or (`|EnumEquality` _movestate "VE_MovingForward") (`|EnumEquality` _movestate "VE_MovingBackward"))
    (bind _asbp_fgcharacter_base (cast `/Game/Blueprints/BP_FGCharacterBase` OtherActor))
    (if (and (`|EnumEquality` (`FGCharacterBase.characterState` _asbp_fgcharacter_base) "VE_Default") (`|EnumEquality` (`FGCharacterBase.moveState` _asbp_fgcharacter_base) "VE_Default"))
      (if (`self.plFacingRight`)
        (`self.K2_AddActorWorldOffset` _asbp_fgcharacter_base (1.2 0.0 0.0) true false)
        (else
          (`self.K2_AddActorWorldOffset` _asbp_fgcharacter_base (-1.2 0.0 0.0) true false))))))

(event `self.HitShaking`)

(event `self.LightFlash`
  (params (flashMultiplier :type "Float (single-precision)"))
  (bind _outactors (`GameplayStatics.GetAllActorsOfClass` "/Script/Engine.SpotLight"))
  (for _array_element _outactors
    (if (`KismetStringLibrary.Contains` (`KismetSystemLibrary.GetDisplayName` _array_element) "BG_ExtraSpotLight_FLOOR")
      (bind (_direction _newtrack_0) (`Timeline|TL_Spotlight` :!via `PlayFromStart`)
        (:`Update`
          (`KismetSystemLibrary.PrintString` (`KismetStringLibrary.Conv_DoubleToString` _newtrack_0))
          (`LightComponent.SetIntensity` (`Light.LightComponent` _array_element) _newtrack_0))))))

(event `CustomEvent`
  (bind _new_track_0 (`self.New Track 0`))
  (for _ (range 1 6)
    (if (== _new_track_0 1.0)
      (`KismetSystemLibrary.PrintString` (`KismetStringLibrary.Conv_DoubleToString` _new_track_0))
      (`self.LaunchCharacter` (0.0 0.0 750.0))
      (else
        (`self.LaunchCharacter` (0.0 0.0 450.0))))))

(event `self.LaunchCharacterTimeline`
  (params (isFacingRight :type Boolean)))

(event `self.IgnorePlayerCollision`
  (params (ignore :type Boolean))
  (bind _capsulecomponent (`self.CapsuleComponent`))
  (if ignore
    (`PrimitiveComponent.SetCollisionResponseToChannel` _capsulecomponent "ECC_WorldDynamic" "ECR_Ignore")
    (else
      (`PrimitiveComponent.SetCollisionResponseToChannel` _capsulecomponent "ECC_WorldDynamic" "ECR_Block"))))

(event `self.ReceiveTick`
  (params (DeltaSeconds :type "Float (single-precision)"))
  (bind (_returnvalue_x _returnvalue_y _returnvalue_z) (`KismetMathLibrary.BreakVector` (`self.K2_GetActorLocation` self)))
  (`|ExecutionSequence`
    (:`then_0`
      (if (or (> _returnvalue_y 0.0) (< _returnvalue_y 0.0))
        (`self.K2_SetActorLocation` (`KismetMathLibrary.MakeVector` _returnvalue_x 0.0 _returnvalue_z))))))

(fn `UserConstructionScript`)