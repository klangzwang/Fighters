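; Fighting game camera director that drives the level's "BattleCamera" actor to frame the left and right characters from the game mode.
; After a short startup delay it spawns two edge actors, repositioned each tick around the fighters to set horizontal limits.
; The camera follows the fighters' midpoint within those limits, otherwise snapping X to zero, with clamped height and separation-based extra depth.
; DoOnce-gated timelines add randomized side-to-side and yaw sway.
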(event `self.ReceiveBeginPlay`
  (`KismetSystemLibrary.Delay` 0.3)
  (bind _asbp_fggame_mode (cast `/Game/Common/BP_FGGameMode` (`GameplayStatics.GetGameMode`)))
  (set `self.FGGameMode` _asbp_fggame_mode)
  (bind _outactors (`GameplayStatics.GetAllActorsOfClass` "/Script/Engine.CameraActor"))
  (for _array_element _outactors
    (if (`KismetStringLibrary.Contains` (`KismetSystemLibrary.GetDisplayName` _array_element) "BattleCamera")
      (set `self.BattleCamera` _array_element)
      (bind _returnvalue (`|SpawnActorFromClass` "/Game/Common/Camera/BP_CameraEdge.BP_CameraEdge_C" (`KismetMathLibrary.MakeTransform` (0.0 0.0 0.0)) "Undefined" "OverrideRootScale" null null))
      (set `self.CamEdgeLeft` _returnvalue)
      (bind _returnvalue_2 (`|SpawnActorFromClass` "/Game/Common/Camera/BP_CameraEdge.BP_CameraEdge_C" (`KismetMathLibrary.MakeTransform` (0.0 0.0 0.0)) "Undefined" "OverrideRootScale" null null))
      (set `self.CamEdgeRight` _returnvalue_2)
      (set `self.hasEdgesSpawned` true))))

(event `self.ReceiveTick`
  (params (DeltaSeconds :type "Float (single-precision)"))
  (if (`self.hasEdgesSpawned`)
    (`self.SetOuterBoundaries`)
    (`self.CameraMovement`)
    (`self.CameraEffectLR`)
    (`self.CameraEffectRA`)))

(event `CameraMovement`
  (bind _fggamemode (`self.FGGameMode`))
  (bind _characterleft (`FGGameMode.CharacterLeft` _fggamemode))
  (bind _characterright (`FGGameMode.CharacterRight` _fggamemode))
  (bind _returnvalue (`KismetMathLibrary.FClamp` (.y (`self.K2_GetActorLocation`)) 520.5 590.5))
  (bind _returnvalue_2 (/ (+ (.x (`self.K2_GetActorLocation` _characterleft)) (.x (`self.K2_GetActorLocation` _characterright))) 2.0))
  (bind _returnvalue_3 (`KismetMathLibrary.FClamp` (/ (/ (+ (.z (`self.K2_GetActorLocation` _characterleft)) (.z (`self.K2_GetActorLocation` _characterright))) 2.0) 1.2) 120.5 130.85))
  (if (and (`KismetSystemLibrary.IsValid` _characterleft) (`KismetSystemLibrary.IsValid` _characterright))
    (bind _canmove (`self.CanStartMoving` _returnvalue_2))
    (if _canmove
      (`self.K2_SetActorLocation` (`self.BattleCamera`) (`KismetMathLibrary.MakeVector` _returnvalue_2 _returnvalue _returnvalue_3) true false)
      (else
        (`self.K2_SetActorLocation` (`self.BattleCamera`) (`KismetMathLibrary.MakeVector` 0.0 _returnvalue _returnvalue_3) true false)))
    (`self.CameraExtraDistance`)))

(event `CameraExtraDistance`
  (bind _fggamemode (`self.FGGameMode`))
  (bind (_returnvalue_x _returnvalue_y _returnvalue_z) (`KismetMathLibrary.BreakVector` (`self.K2_GetActorLocation` (`self.BattleCamera`))))
  (bind _returnvalue (`KismetMathLibrary.FClamp` (`KismetMathLibrary.Abs` (* (- (.x (`self.K2_GetActorLocation` (`FGGameMode.CharacterLeft` _fggamemode))) (.x (`self.K2_GetActorLocation` (`FGGameMode.CharacterRight` _fggamemode)))) 0.12)) 56.0 72.0))
  (set `self.CurrentExtraDistance` _returnvalue)
  (`self.K2_SetActorLocation` (`self.BattleCamera`) (`KismetMathLibrary.MakeVector` _returnvalue_x (+ _returnvalue_y _returnvalue) _returnvalue_z) true false))

(event `CameraEffectLR`
  (bind _cam_leftright (`self.Cam_LeftRight`))
  (`/Engine/EditorBlueprintResources/StandardMacros.DoOnce` false :!label _label
    (:`Completed`
      (switch `int` (`KismetMathLibrary.RandomIntegerInRange` 0 1)
        (:`Default`
          (bind (_direction _newtrack_0) (`Timeline|Cam_LeftRight` :!via `PlayFromStart`)
            (:`Update`
              (`SceneComponent.K2_SetRelativeLocation` (`Actor.RootComponent` (`self.BattleCamera`)) (`KismetMathLibrary.MakeVector` (+ _newtrack_0 (.x (`SceneComponent.RelativeLocation` (`Actor.RootComponent` (`self.BattleCamera`))))) (.y (`SceneComponent.RelativeLocation` (`Actor.RootComponent` (`self.BattleCamera`)))) (.z (`SceneComponent.RelativeLocation` (`Actor.RootComponent` (`self.BattleCamera`))))) false false))
            (:`Finished`
              (goto _label :!via `Reset`))))
        (:`0`
          (`TimelineComponent.ReverseFromEnd` _cam_leftright))
        (:`1`
          (`TimelineComponent.PlayFromStart` _cam_leftright))))))

(event `CameraEffectRA`
  (bind _cam_rotatearound (`self.Cam_RotateAround`))
  (`/Engine/EditorBlueprintResources/StandardMacros.DoOnce` false :!label _label_2
    (:`Completed`
      (switch `int` (`KismetMathLibrary.RandomIntegerInRange` 0 1)
        (:`Default`
          (bind (_direction _newtrack_0) (`Timeline|Cam_RotateAround` :!via `PlayFromStart`)
            (:`Update`
              (`SceneComponent.K2_SetRelativeRotation` (`Actor.RootComponent` (`self.BattleCamera`)) (`KismetMathLibrary.MakeRotator` (.roll (`SceneComponent.RelativeRotation` (`Actor.RootComponent` (`self.BattleCamera`)))) (.pitch (`SceneComponent.RelativeRotation` (`Actor.RootComponent` (`self.BattleCamera`)))) (+ _newtrack_0 (.yaw (`SceneComponent.RelativeRotation` (`Actor.RootComponent` (`self.BattleCamera`)))))) false false))
            (:`Finished`
              (goto _label_2 :!via `Reset`))))
        (:`0`
          (`TimelineComponent.ReverseFromEnd` _cam_rotatearound))
        (:`1`
          (`TimelineComponent.PlayFromStart` _cam_rotatearound))))))

(fn `CanStartMoving`
  (params (CameraMove :type "Float (double-precision)"))
  (returns (canMove :type Boolean))
  (if (> CameraMove (`self.leftMax`))
    (if (< CameraMove (`self.rightMax`))
      (return true)
      (else
        (return false)))
    (else
      (return false))))

(fn `SetOuterBoundaries`
  (bind _returnvalue (- (.x (`self.K2_GetActorLocation` (`FGGameMode.CharacterRight` (`self.FGGameMode`)))) 650.0))
  (bind _returnvalue_2 (- (.x (`self.K2_GetActorLocation` (`FGGameMode.CharacterLeft` (`self.FGGameMode`)))) 650.0))
  (bind _returnvalue_3 (+ (.x (`self.K2_GetActorLocation` (`FGGameMode.CharacterLeft` (`self.FGGameMode`)))) 650.0))
  (bind _returnvalue_4 (+ (.x (`self.K2_GetActorLocation` (`FGGameMode.CharacterRight` (`self.FGGameMode`)))) 650.0))
  (if (`self.hasEdgesSpawned`)
    (if (`FGCharacterBase.plFacingRight` (`FGGameMode.CharacterLeft` (`self.FGGameMode`)))
      (set `self.leftMax` (- _returnvalue 100.0))
      (`self.K2_SetActorLocation` (`self.CamEdgeRight`) (`KismetMathLibrary.MakeVector` _returnvalue (.y (`self.K2_GetActorLocation` (`FGGameMode.CharacterRight` (`self.FGGameMode`)))) (.z (`self.K2_GetActorLocation` (`FGGameMode.CharacterRight` (`self.FGGameMode`))))) false false)
      (set `self.rightMax` (+ _returnvalue_3 100.0))
      (`self.K2_SetActorLocation` (`self.CamEdgeLeft`) (`KismetMathLibrary.MakeVector` _returnvalue_3 (.y (`self.K2_GetActorLocation` (`FGGameMode.CharacterLeft` (`self.FGGameMode`)))) (.z (`self.K2_GetActorLocation` (`FGGameMode.CharacterLeft` (`self.FGGameMode`))))) false false)
      (else
        (set `self.rightMax` (+ _returnvalue_4 100.0))
        (`self.K2_SetActorLocation` (`self.CamEdgeRight`) (`KismetMathLibrary.MakeVector` _returnvalue_4 (.y (`self.K2_GetActorLocation` (`FGGameMode.CharacterRight` (`self.FGGameMode`)))) (.z (`self.K2_GetActorLocation` (`FGGameMode.CharacterRight` (`self.FGGameMode`))))) false false)
        (set `self.leftMax` (- _returnvalue_2 100.0))
        (`self.K2_SetActorLocation` (`self.CamEdgeLeft`) (`KismetMathLibrary.MakeVector` _returnvalue_2 (.y (`self.K2_GetActorLocation` (`FGGameMode.CharacterLeft` (`self.FGGameMode`)))) (.z (`self.K2_GetActorLocation` (`FGGameMode.CharacterLeft` (`self.FGGameMode`))))) false false)))))

(fn `UserConstructionScript`)