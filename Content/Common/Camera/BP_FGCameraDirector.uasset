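; Camera director for a two-player fighting game that frames both characters with the main camera.
; Each tick it moves outer and inner edge actors around the fighters, centres on their midpoint when within edge limits, clamps height and sets FOV from their separation.
; Random timelines add sideways and yaw drift.
; A stage demo event repositions the camera; randomized intro swing shots exist but are never run.
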(event `PlayDemos`)

(event `self.ReceiveBeginPlay`
  (`KismetSystemLibrary.Delay` 0.4)
  (bind _ascamera_actor (cast `CameraActor` (`self.GetMainCamera`)))
  (set `self.CameraMain` _ascamera_actor)
  (`self.SetupCameraMode`)
  (set `self.hasPlayedSwingCam` true))

(event `self.ReceiveTick`
  (params (DeltaSeconds :type "Float (single-precision)"))
  (bind _returnvalue (`GameplayStatics.GetGameMode`))
  (bind _returnvalue_2 (`self.GetMainCamera`))
  (bind (_returnvalue_x _returnvalue_y) (`KismetMathLibrary.BreakVector` (`self.K2_GetActorLocation` _returnvalue_2)))
  (bind _characters (`FGGameMode.Characters` (`self.FGGameMode`)))
  (bind _characters_2 (`FGGameMode.Characters` (`self.FGGameMode`)))
  (bind _output (`|GetArrayItem` _characters_2))
  (bind _output_2 (`|GetArrayItem` _characters_2 1))
  (bind _output_3 (`|GetArrayItem` _characters))
  (bind _output_4 (`|GetArrayItem` _characters 1))
  (bind _returnvalue_3 (/ (+ (.x (`self.K2_GetActorLocation` _output)) (.x (`self.K2_GetActorLocation` _output_2))) 2.0))
  (bind _returnvalue_4 (`KismetMathLibrary.FClamp` (/ (+ (.z (`self.K2_GetActorLocation` _output)) (.z (`self.K2_GetActorLocation` _output_2))) 2.0) 90.0 120.0))
  (bind _asbp_fggame_mode (cast `/Game/Common/BP_FGGameMode` _returnvalue)
    (:`then`
      (set `self.FGGameMode` _asbp_fggame_mode)
      (bind _asbp_fggame_instance (cast `/Game/Common/BP_FGGameInstance` (`GameplayStatics.GetGameInstance`)))
      (bind _returnvalue_5 (`FGGameInstance.hasSpawned` _asbp_fggame_instance))
      (if _returnvalue_5
        (if (and (`self.cameraIsReady`) (`self.hasPlayedSwingCam`)) :!label _label
          (`self.SetOuterBoundaries`)
          (if (`self.hasEdgesSpawned`)
            (`self.CameraEffectLR`)
            (`self.CameraEffectRA`)
            (if (and (`KismetSystemLibrary.IsValid` _output) (`KismetSystemLibrary.IsValid` _output_2))
              (bind _canmove (`self.CanStartMoving` _returnvalue_3))
              (bind _output_get (set `self.canCameraMove` _canmove))
              (if _output_get
                (`self.K2_SetActorLocation` _returnvalue_2 (`KismetMathLibrary.MakeVector` _returnvalue_3 (.y (`self.K2_GetActorLocation` _returnvalue_2)) _returnvalue_4) false false)
                (else
                  (`self.K2_SetActorLocation` _returnvalue_2 (`KismetMathLibrary.MakeVector` _returnvalue_x _returnvalue_y _returnvalue_4) false false)))
              (`self.SetInnerBoundaries` _output_3 _output_4)
              (bind _output_get_2 (set `self.CurrentExtraDistance` (`KismetMathLibrary.FClamp` (`KismetMathLibrary.Abs` (* (- (.x (`self.K2_GetActorLocation` _output_3)) (.x (`self.K2_GetActorLocation` _output_4))) 0.12)) 56.0 72.0)))
              (`CameraComponent.SetFieldOfView` (`CameraActor.CameraComponent` (stale `self.ReceiveBeginPlay` _ascamera_actor)) _output_get_2))))))
    (:`CastFailed`
      (cast `FGGameModeBase` _returnvalue)
      (goto _label))))

(event `CameraEffectLR`
  (bind _cam_leftright (`self.Cam_LeftRight`))
  (bind _rootcomponent (`Actor.RootComponent` (`self.CameraMain`)))
  (`/Engine/EditorBlueprintResources/StandardMacros.DoOnce` false :!label _label_2
    (:`Completed`
      (switch `int` (`KismetMathLibrary.RandomIntegerInRange` 0 1)
        (:`Default`
          (bind (_direction _newtrack_0) (`Timeline|Cam_LeftRight` :!via `PlayFromStart`)
            (:`Update`
              (`SceneComponent.K2_SetRelativeLocation` _rootcomponent (`KismetMathLibrary.MakeVector` (+ _newtrack_0 (.x (`SceneComponent.RelativeLocation` _rootcomponent))) (.y (`SceneComponent.RelativeLocation` _rootcomponent)) (.z (`SceneComponent.RelativeLocation` _rootcomponent))) false false))
            (:`Finished`
              (goto _label_2 :!via `Reset`))))
        (:`0`
          (`TimelineComponent.ReverseFromEnd` _cam_leftright))
        (:`1`
          (`TimelineComponent.PlayFromStart` _cam_leftright))))))

(event `CameraEffectRA`
  (bind _cam_rotatearound (`self.Cam_RotateAround`))
  (bind _rootcomponent (`Actor.RootComponent` (`self.CameraMain`)))
  (`/Engine/EditorBlueprintResources/StandardMacros.DoOnce` false :!label _label_3
    (:`Completed`
      (switch `int` (`KismetMathLibrary.RandomIntegerInRange` 0 1)
        (:`Default`
          (bind (_direction _newtrack_0) (`Timeline|Cam_RotateAround` :!via `PlayFromStart`)
            (:`Update`
              (`SceneComponent.K2_SetRelativeRotation` _rootcomponent (`KismetMathLibrary.MakeRotator` (.roll (`SceneComponent.RelativeRotation` _rootcomponent)) (.pitch (`SceneComponent.RelativeRotation` _rootcomponent)) (+ _newtrack_0 (.yaw (`SceneComponent.RelativeRotation` _rootcomponent)))) false false))
            (:`Finished`
              (goto _label_3 :!via `Reset`))))
        (:`0`
          (`TimelineComponent.ReverseFromEnd` _cam_rotatearound))
        (:`1`
          (`TimelineComponent.PlayFromStart` _cam_rotatearound))))))

(event `DemoStage`
  (`|ExecutionSequence`
    (:`then_0`
      (`KismetSystemLibrary.Delay` 4.0)
      (`TimelineComponent.SetPlayRate` (`self.StageDemo_TL`) 2.0)
      (`Timeline|StageDemo_TL` :!via `PlayFromStart`
        (:`Update`
          (`SceneComponent.K2_SetRelativeLocation` (`Actor.RootComponent` (`self.CameraMain`)) (`KismetMathLibrary.MakeVector` 0.0 600.0 100.0) false false))))
    (:`then_1`
      (`SceneComponent.K2_SetRelativeLocation` (`Actor.RootComponent` (`self.CameraMain`)) (`KismetMathLibrary.MakeVector` 0.0 600.0 100.0) false false))))

(fn `CanStartMoving`
  (params (CameraMove :type "Float (double-precision)"))
  (returns (canMove :type Boolean))
  (if (> CameraMove (`self.EdgeLeftMax`))
    (if (< CameraMove (`self.EdgeRightMax`))
      (return true)
      (else
        (return false)))
    (else
      (return false))))

(fn `SetInnerBoundaries`
  (params (Left :type "FGCharacterBase Object Reference") (Right :type "FGCharacterBase Object Reference"))
  (bind _returnvalue (+ (.x (`self.K2_GetActorLocation` Left)) (`self.EdgeDistance`)))
  (bind _returnvalue_2 (+ (.x (`self.K2_GetActorLocation` Right)) (`self.EdgeDistance`)))
  (bind _returnvalue_3 (- (.x (`self.K2_GetActorLocation` Right)) (`self.EdgeDistance`)))
  (bind _returnvalue_4 (- (.x (`self.K2_GetActorLocation` Left)) (`self.EdgeDistance`)))
  (if (`FGCharacterBase.plFacingRight` Left)
    (set `self.EdgeLeftMax` (- _returnvalue_3 (`self.EdgeMax`)))
    (`self.K2_SetActorLocation` (`self.EdgeInnerRight`) (`KismetMathLibrary.MakeVector` _returnvalue_3 (.y (`self.K2_GetActorLocation` Right)) (.z (`self.K2_GetActorLocation` Right))) false false)
    (set `self.EdgeRightMax` (+ _returnvalue (`self.EdgeMax`)))
    (`self.K2_SetActorLocation` (`self.EdgeInnerLeft`) (`KismetMathLibrary.MakeVector` _returnvalue (.y (`self.K2_GetActorLocation` Left)) (.z (`self.K2_GetActorLocation` Left))) false false)
    (else
      (set `self.EdgeRightMax` (+ _returnvalue_2 (`self.EdgeMax`)))
      (`self.K2_SetActorLocation` (`self.EdgeInnerRight`) (`KismetMathLibrary.MakeVector` _returnvalue_2 (.y (`self.K2_GetActorLocation` Right)) (.z (`self.K2_GetActorLocation` Right))) false false)
      (set `self.EdgeLeftMax` (- _returnvalue_4 (`self.EdgeMax`)))
      (`self.K2_SetActorLocation` (`self.EdgeInnerLeft`) (`KismetMathLibrary.MakeVector` _returnvalue_4 (.y (`self.K2_GetActorLocation` Left)) (.z (`self.K2_GetActorLocation` Left))) false false))))

(fn `SetOuterBoundaries`
  (bind (_returnvalue_x _returnvalue_y _returnvalue_z) (`KismetMathLibrary.BreakVector` (`self.K2_GetActorLocation` (`|GetArrayItem` (`FGGameMode.Characters` (`self.FGGameMode`)) 1))))
  (bind (_returnvalue_x_2 _returnvalue_y_2 _returnvalue_z_2) (`KismetMathLibrary.BreakVector` (`self.K2_GetActorLocation` (`|GetArrayItem` (`FGGameMode.Characters` (`self.FGGameMode`))))))
  (bind _returnvalue (- _returnvalue_x_2 1000.0))
  (bind _returnvalue_2 (+ _returnvalue_x 1000.0))
  (set `self.EdgeLeftMax` (- _returnvalue -200.0))
  (`self.K2_SetActorLocation` (`self.EdgeOuterLeft`) (`KismetMathLibrary.MakeVector` _returnvalue _returnvalue_y_2 _returnvalue_z_2) false false)
  (set `self.EdgeRightMax` (+ _returnvalue_2 -200.0))
  (`self.K2_SetActorLocation` (`self.EdgeOuterRight`) (`KismetMathLibrary.MakeVector` _returnvalue_2 _returnvalue_y _returnvalue_z) false false))

(fn `UserConstructionScript`)