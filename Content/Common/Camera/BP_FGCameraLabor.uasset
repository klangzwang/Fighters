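; BP_FGCameraLabor is a Blueprint that keeps its Cube component in randomized idle motion, apparently as a camera effect.
; Tick calls two DoOnce-gated events, each randomly playing a timeline forward or in reverse and re-arming when it finishes.
; One timeline shifts the Cube along relative X and the other turns its yaw.
; Each update adds the track value to the current transform, so offsets accumulate rather than following the curve absolutely.
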(event `self.ReceiveBeginPlay`)

(event `self.ReceiveTick`
  (params (DeltaSeconds :type "Float (single-precision)"))
  (`self.CameraEffectLR`)
  (`self.CameraEffectRA`))

(event `CameraEffectLR`
  (bind _cube (`self.Cube`))
  (bind _cam_leftright (`self.Cam_LeftRight`))
  (`/Engine/EditorBlueprintResources/StandardMacros.DoOnce` false :!label _label
    (:`Completed`
      (switch `int` (`KismetMathLibrary.RandomIntegerInRange` 0 1)
        (:`Default`
          (bind (_direction _newtrack_0) (`Timeline|Cam_LeftRight` :!via `PlayFromStart`)
            (:`Update`
              (`SceneComponent.K2_SetRelativeLocation` _cube (`KismetMathLibrary.MakeVector` (+ _newtrack_0 (.x (`SceneComponent.RelativeLocation` _cube))) (.y (`SceneComponent.RelativeLocation` _cube)) (.z (`SceneComponent.RelativeLocation` _cube))) false false))
            (:`Finished`
              (goto _label :!via `Reset`))))
        (:`0`
          (`TimelineComponent.ReverseFromEnd` _cam_leftright))
        (:`1`
          (`TimelineComponent.PlayFromStart` _cam_leftright))))))

(event `CameraEffectRA`
  (bind _cube (`self.Cube`))
  (bind _cam_rotatearound (`self.Cam_RotateAround`))
  (`/Engine/EditorBlueprintResources/StandardMacros.DoOnce` false :!label _label_2
    (:`Completed`
      (switch `int` (`KismetMathLibrary.RandomIntegerInRange` 0 1)
        (:`Default`
          (bind (_direction _newtrack_0) (`Timeline|Cam_RotateAround` :!via `PlayFromStart`)
            (:`Update`
              (`SceneComponent.K2_SetRelativeRotation` _cube (`KismetMathLibrary.MakeRotator` (.roll (`SceneComponent.RelativeRotation` _cube)) (.pitch (`SceneComponent.RelativeRotation` _cube)) (+ _newtrack_0 (.yaw (`SceneComponent.RelativeRotation` _cube)))) false false))
            (:`Finished`
              (goto _label_2 :!via `Reset`))))
        (:`0`
          (`TimelineComponent.ReverseFromEnd` _cam_rotatearound))
        (:`1`
          (`TimelineComponent.PlayFromStart` _cam_rotatearound))))))

(fn `UserConstructionScript`)