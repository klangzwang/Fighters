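; Game mode that spawns and wires up the left and right characters of a match.
; After a short delay at BeginPlay, it scans PlayerStarts and spawns BP_CharacterLeft at "PL" tags and BP_CharacterRight at "PR" tags.
; Player controller 0 possesses the left character, while a newly spawned BP_ControllerRight possesses the right one.
; It stores both characters and their controllers, casting the left controller to FGOpenController.
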(event `self.ReceiveBeginPlay`
  (bind _returnvalue (`GameplayStatics.GetPlayerController` 0))
  (`KismetSystemLibrary.Delay` 0.2)
  (bind _outactors (`GameplayStatics.GetAllActorsOfClass` "/Script/Engine.PlayerStart"))
  (for _array_element _outactors
    (bind _playerstarttag (`PlayerStart.PlayerStartTag` _array_element))
    (if (== _playerstarttag "PL")
      (bind _returnvalue_2 (`self.K2_GetActorLocation` _array_element))
      (bind _returnvalue_3 (`|SpawnActorFromClass` "/Game/Blueprints/CharacterLeft/BP_CharacterLeft.BP_CharacterLeft_C" (`KismetMathLibrary.MakeTransform` _returnvalue_2) "Undefined" "MultiplyWithRoot" null null))
      (set `self.CharacterLeft` _returnvalue_3)
      (`Controller.Possess` _returnvalue _returnvalue_3)
      (bind _asfgopen_controller (cast `FGOpenController` _returnvalue))
      (set `self.ControllerLeft` _asfgopen_controller)
      (elif (== _playerstarttag "PR")
        (bind _returnvalue_4 (`|SpawnActorFromClass` "/Game/Blueprints/CharacterRight/BP_CharacterRight.BP_CharacterRight_C" (`KismetMathLibrary.MakeTransform` _returnvalue_2) "Undefined" "MultiplyWithRoot" null null))
        (set `self.CharacterRight` _returnvalue_4)
        (bind _returnvalue_5 (`|SpawnActorFromClass` "/Game/Blueprints/CharacterRight/BP_ControllerRight.BP_ControllerRight_C" (`KismetMathLibrary.MakeTransform` _returnvalue_2) "Undefined" "MultiplyWithRoot" null null))
        (`Controller.Possess` _returnvalue_5 _returnvalue_4)
        (set `self.ControllerRight` _returnvalue_5)))))

(event `self.ReceiveTick`
  (params (DeltaSeconds :type "Float (single-precision)")))

(fn `UserConstructionScript`)