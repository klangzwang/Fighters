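; Game instance Blueprint for a fighting game that seeds the match setup and bootstraps shared systems at startup.
; Init sets hardcoded player, character and stage IDs, then after a short delay creates and initializes the Input Manager and finds the level's Camera Director.
; If ShowDebugWin is set, it passes both, plus the game mode, to a debug widget opened in a separate window.
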(event `self.ReceiveInit`
  (bind _inputmanager (`self.InputManager`))
  (`self.SetPlayerIds` "PLAYER" "PLAYER")
  (`self.SetCharacterIds` "GEN" "MOK")
  (`self.SetStageId` "TRA")
  (`KismetSystemLibrary.Delay` 0.5)
  (`|ExecutionSequence`
    (:`then_0`
      ;[1 1 1] Construct and Init the Input Manager
      (bind _returnvalue (`|GenericCreateObject` "/Game/Common/BP_InputManager.BP_InputManager_C"))
      (set `self.InputManager` _returnvalue)
      (`/Engine/EditorBlueprintResources/StandardMacros.IsValid` _inputmanager
        (:`Is Valid`
          (`InputManager.Initialize` _inputmanager))))
    (:`then_1`
      ;[1 1 1] Setup CameraDirector
      (bind _outactors (`GameplayStatics.GetAllActorsOfClass` "/Game/Common/Camera/BP_FGCameraDirector.BP_FGCameraDirector_C"))
      (set `self.CameraDirector` (`|GetArrayItem` _outactors)))
    (:`then_2`
      (if (`self.showDebugWin`)
        ;[1 1 1] DebugWindow
        (bind _asbp_fggame_mode (cast `/Game/Common/BP_FGGameMode` (`GameplayStatics.GetGameMode`)))
        (bind _asbp_fgcamera_director (cast `/Game/Common/Camera/BP_FGCameraDirector` (`self.CameraDirector`)))
        (bind _returnvalue_2 (`|CreateWidget` "/Game/UI/Debug/WBP_DebugWindow.WBP_DebugWindow_C" null (`self.InputManager`) _asbp_fgcamera_director _asbp_fggame_mode))
        (`FGDebugComponent.OpenAsWindow` (`self.DebugMenuWindow`) _returnvalue_2 "Fighters - Debug" (20.0 20.0) (450.0 450.0) true true true)))))